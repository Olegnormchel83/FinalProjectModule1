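; Default HUD Blueprint that shows the player interface during play and switches to a death screen when the player dies.
; On BeginPlay it caches the level player controller, adds the player interface widget, and binds to the owning character's health component death event.
; On death it removes the interface, shows the death screen, and gives it Game and UI input focus with a visible cursor.
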(event `self.ReceiveBeginPlay`
  (bind _asbp_level_player_controller (cast `/Game/TutorialWork/Core/PlayerController/BP_LevelPlayerController` (`GameplayStatics.GetPlayerController` 0)))
  (set `self.LevelPlayerController` _asbp_level_player_controller)
  (bind _returnvalue (`|CreateWidget` "/Game/TutorialWork/UI/Levels/WBP_PlayerInterface.WBP_PlayerInterface_C" (`self.GetOwningPlayerController`)))
  (bind _output_get (set `self.PlayerInterfaceWidget` _returnvalue))
  (`UserWidget.AddToViewport` _output_get 0)
  (bind _asbp_tutorial_project_character (cast `/Game/TutorialWork/Character/BP_TutorialProjectCharacter` (`self.GetOwningPawn`)))
  (add `/Game/TutorialWork/Blueprints/Components/BP_HealthComponent.OnOwnerDied` (`/Game/TutorialWork/Character/BP_TutorialProjectCharacter.BP_HealthComponent` _asbp_tutorial_project_character) (delegate `OnOwnerDied_Event`)))

(event `OnOwnerDied_Event`
  (`|ExecutionSequence`
    (:`then_0`
      (bind _playerinterfacewidget (`self.PlayerInterfaceWidget`)
        (:`then`
          (`Widget.RemoveFromParent` _playerinterfacewidget))
        (:`else`)))
    (:`then_1`
      (bind _returnvalue (`|CreateWidget` "/Game/TutorialWork/UI/Levels/WBP_DeathScreenWidget.WBP_DeathScreenWidget_C"))
      (bind _output_get (set `self.DeathScreenWidget` _returnvalue))
      (`UserWidget.AddToViewport` _output_get 0)
      (bind _levelplayercontroller (`self.LevelPlayerController`)
        (:`then`
          (`WidgetBlueprintLibrary.SetInputMode_GameAndUIEx` _levelplayercontroller (`self.DeathScreenWidget`))
          (set `PlayerController.bShowMouseCursor` true _levelplayercontroller))
        (:`else`)))))

(fn `UserConstructionScript`)