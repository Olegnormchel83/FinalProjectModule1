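; Player controller that drives the tutorial project character and toggles the pause menu during gameplay.
; On BeginPlay it sets game-only input, adds the Enhanced Input mapping context and caches the possessed character and its movement component.
; Input actions feed control-rotation-relative movement, look and jumping.
; The pause action toggles game pause, input mode and cursor, lazily creating the menu widget and adding it to the viewport when pausing.
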(event `self.ReceiveBeginPlay`
  (`WidgetBlueprintLibrary.SetInputMode_GameOnly` self)
  (set `self.bShowMouseCursor` false)
  (`EnhancedInputSubsystemInterface.AddMappingContext` (subsystem `EnhancedInputLocalPlayerSubsystem`) "/Game/TutorialWork/Core/EnhancedInput/IMC_TutorialProject.IMC_TutorialProject" 0 (struct))
  (bind _asbp_tutorial_project_character (cast `/Game/TutorialWork/Character/BP_TutorialProjectCharacter` (`self.K2_GetPawn`)))
  (bind _output_get (set `self.TutorialProjectCharacter` _asbp_tutorial_project_character))
  (set `self.CharacterMovementComponent` (`Character.CharacterMovement` _output_get)))

(event `EnhancedInput|/Game/TutorialWork/Core/EnhancedInput/Action/IA_TutorialProjectMove`
  (params (ActionValue :type "Vector2D Structure") (ElapsedSeconds :type "Float (double-precision)") (TriggeredSeconds :type "Float (double-precision)") (InputAction :type "InputAction Object Reference" :default "/Game/TutorialWork/Core/EnhancedInput/Action/IA_TutorialProjectMove.IA_TutorialProjectMove"))
  (bind (_returnvalue_roll _returnvalue_pitch _returnvalue_yaw) (`KismetMathLibrary.BreakRotator` (`self.GetControlRotation`)))
  (:`Triggered`
    (bind _charactermovementcomponent (`self.CharacterMovementComponent`)
      (:`then`
        (`|ExecutionSequence`
          (:`then_0`
            (`PawnMovementComponent.AddInputVector` _charactermovementcomponent (* ActionValue_Y (`KismetMathLibrary.GetForwardVector` (`KismetMathLibrary.MakeRotator` 0.0 0.0 _returnvalue_yaw))) false))
          (:`then_1`
            (`PawnMovementComponent.AddInputVector` _charactermovementcomponent (* ActionValue_X (`KismetMathLibrary.GetRightVector` (`KismetMathLibrary.MakeRotator` _returnvalue_roll 0.0 _returnvalue_yaw))) false))))
      (:`else`))))

(event `EnhancedInput|/Game/TutorialWork/Core/EnhancedInput/Action/IA_TutorialProjectLook`
  (params (ActionValue :type "Vector2D Structure") (ElapsedSeconds :type "Float (double-precision)") (TriggeredSeconds :type "Float (double-precision)") (InputAction :type "InputAction Object Reference" :default "/Game/TutorialWork/Core/EnhancedInput/Action/IA_TutorialProjectLook.IA_TutorialProjectLook"))
  (:`Triggered`
    (`self.AddYawInput` ActionValue_X)
    (`self.AddPitchInput` ActionValue_Y)))

(event `EnhancedInput|/Game/TutorialWork/Core/EnhancedInput/Action/IA_TutorialProjectJump`
  (params (ActionValue :type Boolean) (ElapsedSeconds :type "Float (double-precision)") (TriggeredSeconds :type "Float (double-precision)") (InputAction :type "InputAction Object Reference" :default "/Game/TutorialWork/Core/EnhancedInput/Action/IA_TutorialProjectJump.IA_TutorialProjectJump"))
  (:`Triggered`
    (bind _tutorialprojectcharacter (`self.TutorialProjectCharacter`)
      (:`then`
        (`Character.Jump` _tutorialprojectcharacter))
      (:`else`)))
  (:`Completed`
    (`Character.StopJumping` _tutorialprojectcharacter)))

(event `EnhancedInput|/Game/TutorialWork/Core/EnhancedInput/Action/IA_TutorialProjectPauseMenu`
  (params (ActionValue :type Boolean) (ElapsedSeconds :type "Float (double-precision)") (TriggeredSeconds :type "Float (double-precision)") (InputAction :type "InputAction Object Reference" :default "/Game/TutorialWork/Core/EnhancedInput/Action/IA_TutorialProjectPauseMenu.IA_TutorialProjectPauseMenu"))
  (:`Triggered`
    (if (`GameplayStatics.IsGamePaused`)
      (`GameplayStatics.SetGamePaused` false)
      (`WidgetBlueprintLibrary.SetInputMode_GameOnly` null)
      (set `self.bShowMouseCursor` false)
      (else
        (`GameplayStatics.SetGamePaused` true)
        (`self.PasuMenuWidget`
          (:`then`
            _)
          (:`else`
            (bind _returnvalue (`|CreateWidget` "/Game/TutorialWork/UI/Levels/WBP_PauseMenuWidget.WBP_PauseMenuWidget_C" self))
            (bind _output_get (set `self.PasuMenuWidget` _returnvalue))))
        (`UserWidget.AddToViewport` _output_get 0)
        (`WidgetBlueprintLibrary.SetInputMode_GameAndUIEx` self _output_get)
        (set `self.bShowMouseCursor` true)))))

(fn `UserConstructionScript`)