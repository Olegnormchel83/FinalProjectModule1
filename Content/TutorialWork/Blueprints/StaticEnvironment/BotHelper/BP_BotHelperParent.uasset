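; BP_BotHelperParent is a base helper-bot actor that reveals a widget when the player character comes near it.
; On BeginPlay it caches the player character and its class, then hides the widget.
; Box overlap begin shows the widget and plays the C_BotHelper sound at the actor's location; overlap end hides the widget again.
; Both overlap handlers react only to actors of the cached player class.
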(event `self.ReceiveBeginPlay`
  (bind _asbp_tutorial_project_character (cast `/Game/TutorialWork/Character/BP_TutorialProjectCharacter` (`GameplayStatics.GetPlayerPawn` 0)))
  (bind _output_get (set `self.TutorialProjectCharacter` _asbp_tutorial_project_character))
  (set `self.PlayerCharacterClass` (`GameplayStatics.GetObjectClass` _output_get))
  (`SceneComponent.SetVisibility` (`self.Widget`) false false))

(event `self.Box.OnComponentBeginOverlap`
  (params (OverlappedComponent :type "PrimitiveComponent Object Reference") (OtherActor :type "Actor Object Reference") (OtherComp :type "PrimitiveComponent Object Reference") (OtherBodyIndex :type Integer) (bFromSweep :type Boolean) (SweepResult :type "HitResult Structure (by ref)"))
  (if (`GameplayStatics.ObjectIsA` OtherActor (`self.PlayerCharacterClass`))
    (`SceneComponent.SetVisibility` (`self.Widget`) true false)
    (`GameplayStatics.PlaySoundAtLocation` "/Game/TutorialWork/Sounds/Cues/C_BotHelper.C_BotHelper" (`self.K2_GetActorLocation`) (struct) 1.0 1.0 0.0 null null null null)))

(event `self.Box.OnComponentEndOverlap`
  (params (OverlappedComponent :type "PrimitiveComponent Object Reference") (OtherActor :type "Actor Object Reference") (OtherComp :type "PrimitiveComponent Object Reference") (OtherBodyIndex :type Integer))
  (if (`GameplayStatics.ObjectIsA` OtherActor (`self.PlayerCharacterClass`))
    (`SceneComponent.SetVisibility` (`self.Widget`) false false)))

(fn `UserConstructionScript`)