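; BP_HealthComponent is a component that tracks its owning actor's health and signals when that owner dies.
; On BeginPlay it binds to the owner's OnTakeAnyDamage event and sets health from DefaultHealth.
; Incoming damage is subtracted and clamped between zero and current health, so negative damage cannot heal.
; It calls the OnOwnerDied dispatcher whenever a hit leaves health at zero, including repeat hits after death.
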(event `self.ReceiveBeginPlay`
  (add `Actor.OnTakeAnyDamage` (`self.GetOwner`) (delegate `OnTakeAnyDamage_Event`))
  (`self.SetHealth` (`self.DefaultHealth`)))

(event `OnTakeAnyDamage_Event`
  (params (DamagedActor :type "Actor Object Reference") (Damage :type "Float (single-precision)") (DamageType :type "DamageType Object Reference") (InstigatedBy :type "Controller Object Reference") (DamageCauser :type "Actor Object Reference"))
  (`self.GetDamage` Damage))

(fn `GetDamage`
  (params (InDamage :type "Float (double-precision)"))
  (bind _health (`self.GetHealth`))
  (`self.SetHealth` (`KismetMathLibrary.FClamp` (- _health InDamage) 0.0 _health))
  (if (<= (`self.GetHealth`) 0.0)
    (`self.OnOwnerDied`)))

(fn `GetDefaultHealth`
  (returns (DefaultHealth :type "Float (double-precision)"))
  (return (`self.DefaultHealth`)))

(fn `GetHealth`
  (returns (Health :type "Float (double-precision)"))
  (return (`self.Health`)))

(fn `SetDefaultHealth`
  (params (NewDefaultHealth :type "Float (double-precision)"))
  (set `self.DefaultHealth` NewDefaultHealth))

(fn `SetHealth`
  (params (NewHealth :type "Float (double-precision)"))
  (set `self.Health` NewHealth))