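; BP_MovePlatform is a platform actor meant to shuttle between MinLimit and MaxLimit along world X or Y, chosen by MovementX.
; BeginPlay sets the initial positive Direction, and Tick calls XMovement or YMovement to compute a delta-time scaled step and reverse Direction at either limit.
; YMovement applies only steps inside the limits.
; XMovement applies only steps reaching a limit, so it stays still between them.
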(event `self.ReceiveBeginPlay`
  (if (`self.MovementX`)
    (set `self.Direction` (1.0 0.0 0.0))
    (else
      (set `self.Direction` (0.0 1.0 0.0)))))

(event `self.ReceiveTick`
  (params (DeltaSeconds :type "Float (single-precision)"))
  (if (`self.MovementX`)
    (`self.XMovement`)
    (else
      (`self.YMovement`))))

(fn `UserConstructionScript`)

(fn `XMovement`
  (bind _returnvalue_x (`KismetMathLibrary.BreakVector` (`self.K2_GetActorLocation`)))
  (bind (_returnvalue_x_2 _returnvalue_y _returnvalue_z) (`KismetMathLibrary.BreakVector` (`self.K2_GetActorLocation`)))
  (bind _returnvalue_x_3 (`KismetMathLibrary.BreakVector` (* (* (`GameplayStatics.GetWorldDeltaSeconds`) (`self.Speed`)) (`self.Direction`))))
  (bind _output_get (set `self.NewCoord` (+ _returnvalue_x _returnvalue_x_3)))
  (if (>= _output_get (`self.MaxLimit`))
    (set `self.Direction` (-1.0 0.0 0.0))
    (`self.K2_SetActorLocation` (`KismetMathLibrary.MakeVector` (`self.NewCoord`) _returnvalue_y _returnvalue_z) :!label _label)
    (elif (<= _output_get (`self.MinLimit`))
      (set `self.Direction` (1.0 0.0 0.0))
      (goto _label))))

(fn `YMovement`
  (bind (_returnvalue_x _returnvalue_y) (`KismetMathLibrary.BreakVector` (`self.K2_GetActorLocation`)))
  (bind (_returnvalue_x_2 _returnvalue_y_2 _returnvalue_z) (`KismetMathLibrary.BreakVector` (`self.K2_GetActorLocation`)))
  (bind (_returnvalue_x_3 _returnvalue_y_3) (`KismetMathLibrary.BreakVector` (* (* (`GameplayStatics.GetWorldDeltaSeconds`) (`self.Speed`)) (`self.Direction`))))
  (bind _output_get (set `self.NewCoord` (+ _returnvalue_y _returnvalue_y_3)))
  (if (>= _output_get (`self.MaxLimit`))
    (set `self.Direction` (0.0 -1.0 0.0))
    (elif (<= _output_get (`self.MinLimit`))
      (set `self.Direction` (0.0 1.0 0.0))
      (else
        (`self.K2_SetActorLocation` (`KismetMathLibrary.MakeVector` _returnvalue_x_2 (`self.NewCoord`) _returnvalue_z))))))