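; Interaction door puzzle in which the player must turn a target green before the door will open.
; Five colored trigger boxes each repaint GreenTarget on player overlap, then CheckSolution compares its material to green to set DoorCanBeOpened.
; When the player enters the door's box while unlocked, a sound plays and a timeline slides the door along Z.
; On finish, the door and its trigger are destroyed.
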(event `self.ReceiveBeginPlay`
  (`parent.ReceiveBeginPlay`)
  (set `self.bDoorCanBeOpened` false)
  (set `self.bDoorIsOpened` false))

(event `self.GreenBoxCollision.OnComponentBeginOverlap`
  (params (OverlappedComponent :type "PrimitiveComponent Object Reference") (OtherActor :type "Actor Object Reference") (OtherComp :type "PrimitiveComponent Object Reference") (OtherBodyIndex :type Integer) (bFromSweep :type Boolean) (SweepResult :type "HitResult Structure (by ref)"))
  (if (`GameplayStatics.ObjectIsA` OtherActor (`self.PlayerCharacterClass`))
    (if (not (`self.bDoorIsOpened`))
      (`PrimitiveComponent.SetMaterial` (`self.Green(target)`) 0 "/Game/TutorialWork/Materials/MediumDifficultyDoor/MI_GreenColor.MI_GreenColor")
      (bind _right (`self.CheckSolution` :!label _label))
      (set `self.bDoorCanBeOpened` _right))))

(event `self.RedBoxCollision.OnComponentBeginOverlap`
  (params (OverlappedComponent :type "PrimitiveComponent Object Reference") (OtherActor :type "Actor Object Reference") (OtherComp :type "PrimitiveComponent Object Reference") (OtherBodyIndex :type Integer) (bFromSweep :type Boolean) (SweepResult :type "HitResult Structure (by ref)"))
  (if (`GameplayStatics.ObjectIsA` OtherActor (`self.PlayerCharacterClass`))
    (if (not (`self.bDoorIsOpened`))
      (`PrimitiveComponent.SetMaterial` (`self.Green(target)`) 0 "/Game/TutorialWork/Materials/MediumDifficultyDoor/MI_RedColor.MI_RedColor")
      (goto _label))))

(event `self.OrangeBoxCollision.OnComponentBeginOverlap`
  (params (OverlappedComponent :type "PrimitiveComponent Object Reference") (OtherActor :type "Actor Object Reference") (OtherComp :type "PrimitiveComponent Object Reference") (OtherBodyIndex :type Integer) (bFromSweep :type Boolean) (SweepResult :type "HitResult Structure (by ref)"))
  (if (`GameplayStatics.ObjectIsA` OtherActor (`self.PlayerCharacterClass`))
    (if (not (`self.bDoorIsOpened`))
      (`PrimitiveComponent.SetMaterial` (`self.Green(target)`) 0 "/Game/TutorialWork/Materials/MediumDifficultyDoor/MI_OrangeColor.MI_OrangeColor")
      (goto _label))))

(event `self.BlueBoxCollision.OnComponentBeginOverlap`
  (params (OverlappedComponent :type "PrimitiveComponent Object Reference") (OtherActor :type "Actor Object Reference") (OtherComp :type "PrimitiveComponent Object Reference") (OtherBodyIndex :type Integer) (bFromSweep :type Boolean) (SweepResult :type "HitResult Structure (by ref)"))
  (if (`GameplayStatics.ObjectIsA` OtherActor (`self.PlayerCharacterClass`))
    (if (not (`self.bDoorIsOpened`))
      (`PrimitiveComponent.SetMaterial` (`self.Green(target)`) 0 "/Game/TutorialWork/Materials/MediumDifficultyDoor/MI_BlueColor.MI_BlueColor")
      (goto _label))))

(event `self.CyanBoxCollision.OnComponentBeginOverlap`
  (params (OverlappedComponent :type "PrimitiveComponent Object Reference") (OtherActor :type "Actor Object Reference") (OtherComp :type "PrimitiveComponent Object Reference") (OtherBodyIndex :type Integer) (bFromSweep :type Boolean) (SweepResult :type "HitResult Structure (by ref)"))
  (if (`GameplayStatics.ObjectIsA` OtherActor (`self.PlayerCharacterClass`))
    (if (not (`self.bDoorIsOpened`))
      (`PrimitiveComponent.SetMaterial` (`self.Green(target)`) 0 "/Game/TutorialWork/Materials/MediumDifficultyDoor/MI_CyanColor.MI_CyanColor")
      (goto _label))))

(event `self.Box.OnComponentBeginOverlap`
  (params (OverlappedComponent :type "PrimitiveComponent Object Reference") (OtherActor :type "Actor Object Reference") (OtherComp :type "PrimitiveComponent Object Reference") (OtherBodyIndex :type Integer) (bFromSweep :type Boolean) (SweepResult :type "HitResult Structure (by ref)"))
  (bind _door (`self.Door`))
  (bind (_relativelocation_x _relativelocation_y) (`KismetMathLibrary.BreakVector` (`SceneComponent.RelativeLocation` _door)))
  (if (`GameplayStatics.ObjectIsA` OtherActor (`self.PlayerCharacterClass`))
    (if (`self.bDoorIsOpened`)
      _
      (elif (`self.bDoorCanBeOpened`)
        (`|ExecutionSequence`
          (:`then_0`
            (`GameplayStatics.PlaySoundAtLocation` "/Game/TutorialWork/Sounds/Cues/C_OpenDoor.C_OpenDoor" (`self.K2_GetActorLocation`) (struct) 1.0 1.0 0.0 null null null null))
          (:`then_1`
            (bind (_direction _zoffset) (`Timeline|Timeline` :!via `PlayFromStart`)
              (:`Update`
                (`SceneComponent.K2_SetRelativeLocation` _door (`KismetMathLibrary.MakeVector` _relativelocation_x _relativelocation_y (`KismetMathLibrary.MapRangeClamped` _zoffset 0.0 1.0 0.0 -300.0)) false false)
                (set `self.bDoorIsOpened` true))
              (:`Finished`
                (`ActorComponent.K2_DestroyComponent` (`self.Door`))
                (`ActorComponent.K2_DestroyComponent` (`self.Box`))))))))))

(fn `CheckSolution`
  (returns (Right :type Boolean))
  (if (== (`PrimitiveComponent.GetMaterial` (`self.Green(target)`) 0) "/Game/TutorialWork/Materials/MediumDifficultyDoor/MI_GreenColor.MI_GreenColor")
    (return true)
    (else
      (return false))))

(fn `UserConstructionScript`
  (`parent.UserConstructionScript`))