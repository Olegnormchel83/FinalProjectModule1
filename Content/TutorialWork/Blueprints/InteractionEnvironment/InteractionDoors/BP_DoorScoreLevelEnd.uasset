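; BP_DoorScoreLevelEnd is a door that opens for the player once no BP_Coin actors remain in the level.
; When the player overlaps its Box trigger, it checks for remaining coins and, if none are left, plays a sound and sets a flag against retriggering.
; A Timeline lowers the Door component along Z, then destroys both the door and trigger when finished.
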(event `self.ReceiveBeginPlay`
  (`parent.ReceiveBeginPlay`)
  (set `self.bDoorIsOpened` false))

(event `self.Box.OnComponentBeginOverlap`
  (params (OverlappedComponent :type "PrimitiveComponent Object Reference") (OtherActor :type "Actor Object Reference") (OtherComp :type "PrimitiveComponent Object Reference") (OtherBodyIndex :type Integer) (bFromSweep :type Boolean) (SweepResult :type "HitResult Structure (by ref)"))
  (bind _door (`self.Door`))
  (bind (_relativelocation_x _relativelocation_y) (`KismetMathLibrary.BreakVector` (`SceneComponent.RelativeLocation` _door)))
  (if (`GameplayStatics.ObjectIsA` OtherActor (`self.PlayerCharacterClass`))
    (if (not (`self.bDoorIsOpened`))
      (bind _outactors (`GameplayStatics.GetAllActorsOfClass` "/Game/TutorialWork/Blueprints/InteractionEnvironment/Coins/BP_Coin.BP_Coin_C"))
      (if (`KismetArrayLibrary.Array_IsEmpty` _outactors)
        (`|ExecutionSequence`
          (:`then_0`
            (`GameplayStatics.PlaySoundAtLocation` "/Game/TutorialWork/Sounds/Cues/C_OpenDoor.C_OpenDoor" (`self.K2_GetActorLocation`) (struct) 1.0 1.0 0.0 null null null null))
          (:`then_1`
            (bind (_direction _zoffset) (`Timeline|Timeline` :!via `PlayFromStart`)
              (:`Update`
                (`SceneComponent.K2_SetRelativeLocation` _door (`KismetMathLibrary.MakeVector` _relativelocation_x _relativelocation_y (`KismetMathLibrary.MapRangeClamped` _zoffset 0.0 1.0 0.0 -300.0)) false false))
              (:`Finished`
                (`ActorComponent.K2_DestroyComponent` (`self.Door`))
                (`ActorComponent.K2_DestroyComponent` (`self.Box`)))))
          (:`then_2`
            (set `self.bDoorIsOpened` true)))))))

(fn `UserConstructionScript`
  (`parent.UserConstructionScript`))