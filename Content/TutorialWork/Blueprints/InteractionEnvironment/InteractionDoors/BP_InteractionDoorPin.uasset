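; Interactable PIN-locked door that shows an interaction tip while the player character overlaps its pin collision.
; Interacting opens a PIN entry widget with UI-only input and a visible cursor.
; A getter exposes the correct PIN, but checking happens outside this Blueprint.
; The OpenDoor event destroys the collision components, plays a sound and lowers the door along a timeline before destroying it.
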(event `self.ReceiveBeginPlay`
  (`parent.ReceiveBeginPlay`))

(event `self.SM_PinCollision.OnComponentBeginOverlap`
  (params (OverlappedComponent :type "PrimitiveComponent Object Reference") (OtherActor :type "Actor Object Reference") (OtherComp :type "PrimitiveComponent Object Reference") (OtherBodyIndex :type Integer) (bFromSweep :type Boolean) (SweepResult :type "HitResult Structure (by ref)"))
  (if (`GameplayStatics.ObjectIsA` OtherActor (`self.PlayerCharacterClass`))
    (bind _returnvalue (`|CreateWidget` "/Game/TutorialWork/UI/InteractWidgets/WBP_InteractTip.WBP_InteractTip_C"))
    (bind _output_get (set `self.InteractTipWodget` _returnvalue))
    (`UserWidget.AddToViewport` _output_get 0)))

(event `self.SM_PinCollision.OnComponentEndOverlap`
  (params (OverlappedComponent :type "PrimitiveComponent Object Reference") (OtherActor :type "Actor Object Reference") (OtherComp :type "PrimitiveComponent Object Reference") (OtherBodyIndex :type Integer))
  (if (`GameplayStatics.ObjectIsA` OtherActor (`self.PlayerCharacterClass`))
    (bind _interacttipwodget (`self.InteractTipWodget`)
      (:`then`
        (`Widget.RemoveFromParent` _interacttipwodget)
        (set `self.InteractTipWodget` null))
      (:`else`))))

(event `/Game/TutorialWork/Blueprints/Interfaces/BPI_Interactable.Interact`
  (bind _returnvalue (`GameplayStatics.GetPlayerController` 0))
  (bind _returnvalue_2 (`|CreateWidget` "/Game/TutorialWork/UI/InteractWidgets/WBP_PinWidget.WBP_PinWidget_C"))
  (bind _output_get (set `self.PinWidget` _returnvalue_2))
  (`UserWidget.AddToViewport` _output_get 0)
  (`WidgetBlueprintLibrary.SetInputMode_UIOnlyEx` _returnvalue (`self.PinWidget`) "DoNotLock" true)
  (set `PlayerController.bShowMouseCursor` true _returnvalue))

(event `OpenDoor`
  (bind _door (`self.Door`))
  (bind (_relativelocation_x _relativelocation_y) (`KismetMathLibrary.BreakVector` (`SceneComponent.RelativeLocation` _door)))
  (`ActorComponent.K2_DestroyComponent` (`self.SM_PinCollision`))
  (`ActorComponent.K2_DestroyComponent` (`self.Box`))
  (`|ExecutionSequence`
    (:`then_0`
      (`GameplayStatics.PlaySoundAtLocation` "/Game/TutorialWork/Sounds/Cues/C_OpenDoor.C_OpenDoor" (`self.K2_GetActorLocation`) (struct) 1.0 1.0 0.0 null null null null))
    (:`then_1`
      (bind (_direction _zoffset) (`Timeline|OpenDoorTimeline` :!via `PlayFromStart`)
        (:`Update`
          (`SceneComponent.K2_SetRelativeLocation` _door (`KismetMathLibrary.MakeVector` _relativelocation_x _relativelocation_y (`KismetMathLibrary.MapRangeClamped` _zoffset 0.0 1.0 0.0 -300.0)) false false))
        (:`Finished`
          (`ActorComponent.K2_DestroyComponent` (`self.Door`)))))))

(fn `GetCorrecrPin`
  (returns (CorrentPin :type "Array of Integer"))
  (return (`self.CorrentPin`)))

(fn `UserConstructionScript`
  (`parent.UserConstructionScript`))