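; Timed explosive actor that arms when an actor implementing BPI_Damageable overlaps its sphere.
; Overlap starts the explosion timer, plays a bomb sound and runs a timeline tinting the point light, whose updates also set a looping Blink timer.
; Blink replays a second timeline to pulse the light color.
; Explode applies radial damage at twice Radius, spawns explosion effects and sound, clears both timers and destroys the actor.
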(event `self.ReceiveBeginPlay`
  (`parent.ReceiveBeginPlay`))

(event `Blink`
  (bind (_direction _blinktime) (`Timeline|Blinking` :!via `PlayFromStart`)
    (:`Update`
      (`LightComponent.SetLightColor` (`self.PointLight`) (make `LinearColor` 1.0 _blinktime _blinktime 1.0) true))))

(event `self.Sphere.OnComponentBeginOverlap`
  (params (OverlappedComponent :type "PrimitiveComponent Object Reference") (OtherActor :type "Actor Object Reference") (OtherComp :type "PrimitiveComponent Object Reference") (OtherBodyIndex :type Integer) (bFromSweep :type Boolean) (SweepResult :type "HitResult Structure (by ref)"))
  (if (`KismetSystemLibrary.DoesImplementInterface` OtherActor "/Game/TutorialWork/Blueprints/Interfaces/BPI_Damageable.BPI_Damageable_C")
    (bind _returnvalue (`KismetSystemLibrary.K2_SetTimerDelegate` (delegate `Explode`) (`self.TimeToExplode`)))
    (set `self.ExplodeTimerHandle` _returnvalue)
    (`GameplayStatics.PlaySoundAtLocation` "/Game/TutorialWork/Sounds/Cues/C_TimerBomb.C_TimerBomb" (`self.K2_GetActorLocation`) (struct) 1.0 1.0 0.0 null null null null)
    (bind (_direction _blinktime) (`Timeline|Timeline` :!via `PlayFromStart`)
      (:`Update`
        (bind _returnvalue_2 (`KismetMathLibrary.MapRangeClamped` _blinktime 0.0 0.4 0.0 1.0))
        (`LightComponent.SetLightColor` (`self.PointLight`) (make `LinearColor` 1.0 _returnvalue_2 _returnvalue_2 1.0) true)
        (bind _returnvalue_3 (`KismetSystemLibrary.K2_SetTimerDelegate` (delegate `Blink`) 0.4 true))
        (set `self.BlinkingTimerHandle` _returnvalue_3)))))

(event `Explode`
  (bind _returnvalue (`self.K2_GetActorLocation`))
  (`GameplayStatics.ApplyRadialDamage` :`BaseDamage` (`self.Damage`) :`Origin` _returnvalue :`DamageRadius` (* (`self.Radius`) 2.0) :`DamageCauser` self :`InstigatedByController` null :`bDoFullDamage` (`self.DoFullDamage`))
  (`GameplayStatics.SpawnEmitterAtLocation` "/Game/TutorialWork/Blueprints/DamageItems/Particles/P_Explosion.P_Explosion" _returnvalue)
  (`GameplayStatics.PlaySoundAtLocation` "/Game/TutorialWork/Sounds/Cues/C_Explosion.C_Explosion" _returnvalue (struct) 1.0 1.0 0.0 null null null null)
  (`KismetSystemLibrary.K2_ClearAndInvalidateTimerHandle` (`self.BlinkingTimerHandle`))
  (`KismetSystemLibrary.K2_ClearAndInvalidateTimerHandle` (`self.ExplodeTimerHandle`))
  (`self.K2_DestroyActor`))

(fn `UserConstructionScript`
  (`parent.UserConstructionScript`))