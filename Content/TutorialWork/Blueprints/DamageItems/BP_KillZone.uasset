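; BP_KillZone is a damage volume that kills damageable actors entering it.
; When its Box component begins overlapping an actor implementing BPI_Damageable, it spawns a lightning particle effect and hit sound at that actor's location.
; It then applies a very large damage amount through ApplyDamage with itself as the causer; the interface serves only as a filter.
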(event `self.Box.OnComponentBeginOverlap`
  (params (OverlappedComponent :type "PrimitiveComponent Object Reference") (OtherActor :type "Actor Object Reference") (OtherComp :type "PrimitiveComponent Object Reference") (OtherBodyIndex :type Integer) (bFromSweep :type Boolean) (SweepResult :type "HitResult Structure (by ref)"))
  (if (`KismetSystemLibrary.DoesImplementInterface` OtherActor "/Game/TutorialWork/Blueprints/Interfaces/BPI_Damageable.BPI_Damageable_C")
    (`GameplayStatics.SpawnEmitterAtLocation` "/Game/TutorialWork/Blueprints/DamageItems/Particles/P_ky_lightning3.P_ky_lightning3" (`self.K2_GetActorLocation` OtherActor))
    (`GameplayStatics.PlaySoundAtLocation` "/Game/TutorialWork/Sounds/Cues/C_LightningHit.C_LightningHit" (`self.K2_GetActorLocation` OtherActor) (struct) 1.0 1.0 0.0 null null null null)
    (`GameplayStatics.ApplyDamage` OtherActor 1000.0 null self)))

(fn `UserConstructionScript`
  (`parent.UserConstructionScript`))