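; BP_GUN is an automatic weapon actor that repeatedly fires BP_Screwdriver projectiles without any input.
; On BeginPlay a looping timer calls Attack at the AttackSpeedSec interval.
; Each Attack spawns an enlarged screwdriver at the SceneComponent's world location and rotation, ignoring collision.
; A valid spawn gets a short lifespan and the gun's ProjectileDamage, and a shot sound plays at the gun's location.
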(event `self.ReceiveBeginPlay`
  (`KismetSystemLibrary.K2_SetTimerDelegate` (delegate `Attack`) (`self.AttackSpeed(sec)`) true))

(event `Attack`
  (bind _scenecomponent (`self.SceneComponent`))
  (bind (_returnvalue_roll _returnvalue_pitch _returnvalue_yaw) (`KismetMathLibrary.BreakRotator` (`SceneComponent.K2_GetComponentRotation` _scenecomponent)))
  (bind _returnvalue (`|SpawnActorFromClass` "/Game/TutorialWork/Blueprints/DamageItems/BP_Screwdriver.BP_Screwdriver_C" (`KismetMathLibrary.MakeTransform` (`SceneComponent.K2_GetComponentLocation` _scenecomponent) (`KismetMathLibrary.MakeRotator` _returnvalue_roll _returnvalue_pitch _returnvalue_yaw) (2.0 2.0 2.0)) "AlwaysSpawn" "MultiplyWithRoot" null null))
  (`/Engine/EditorBlueprintResources/StandardMacros.IsValid` _returnvalue
    (:`Is Valid`
      (`self.SetLifeSpan` _returnvalue 1.0)
      (set `/Game/TutorialWork/Blueprints/DamageItems/BP_DamageItemParent.Damage` (`self.ProjectileDamage`) _returnvalue)
      (`GameplayStatics.PlaySoundAtLocation` "/Game/TutorialWork/Sounds/Cues/C_Shot.C_Shot" (`self.K2_GetActorLocation`) (struct) 1.0 1.0 0.0 null null null null))))

(fn `UserConstructionScript`)