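; BP_Fire is a fire hazard that repeatedly damages the area within its sphere while triggered.
; When an actor implementing BPI_Damageable begins overlapping the Sphere, a fast looping timer starts calling FireDamage.
; FireDamage applies radial damage from the actor's location, using the Sphere's radius.
; End overlap by a damageable actor clears the timer through a single stored handle, which each new overlap overwrites.
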(event `self.Sphere.OnComponentBeginOverlap`
  (params (OverlappedComponent :type "PrimitiveComponent Object Reference") (OtherActor :type "Actor Object Reference") (OtherComp :type "PrimitiveComponent Object Reference") (OtherBodyIndex :type Integer) (bFromSweep :type Boolean) (SweepResult :type "HitResult Structure (by ref)"))
  (if (`KismetSystemLibrary.DoesImplementInterface` OtherActor "/Game/TutorialWork/Blueprints/Interfaces/BPI_Damageable.BPI_Damageable_C")
    (bind _returnvalue (`KismetSystemLibrary.K2_SetTimerDelegate` (delegate `FireDamage`) 0.1 true))
    (set `self.FireDamageTimerHandle` _returnvalue)))

(event `FireDamage`
  (`GameplayStatics.ApplyRadialDamage` :`BaseDamage` (`self.Damage`) :`Origin` (`self.K2_GetActorLocation`) :`DamageRadius` (`SphereComponent.SphereRadius` (`self.Sphere`)) :`DamageCauser` self :`InstigatedByController` null))

(event `self.Sphere.OnComponentEndOverlap`
  (params (OverlappedComponent :type "PrimitiveComponent Object Reference") (OtherActor :type "Actor Object Reference") (OtherComp :type "PrimitiveComponent Object Reference") (OtherBodyIndex :type Integer))
  (if (`KismetSystemLibrary.DoesImplementInterface` OtherActor "/Game/TutorialWork/Blueprints/Interfaces/BPI_Damageable.BPI_Damageable_C")
    (`KismetSystemLibrary.K2_ClearAndInvalidateTimerHandle` (`self.FireDamageTimerHandle`))))

(fn `UserConstructionScript`
  (`parent.UserConstructionScript`))