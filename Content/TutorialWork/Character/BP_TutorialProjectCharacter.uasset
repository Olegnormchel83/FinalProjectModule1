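; BP_TutorialProjectCharacter is a character Blueprint that handles interaction, score, coin collection and death.
; Capsule overlaps store actors implementing BPI_Interactable as CurrentInteract, which the interact input messages; no end-overlap handler clears it.
; AddScore increments the score on the cached player state, while CollectCoin fires a dispatcher.
; When BP_HealthComponent reports death, it disables input and capsule collision, ragdolls the mesh and sets a short lifespan.
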(event `self.ReceiveBeginPlay`
  (bind _asbp_tutorial_project_player_state (cast `/Game/TutorialWork/Core/PlayerState/BP_TutorialProjectPlayerState` (`GameplayStatics.GetPlayerState` 0)))
  (set `self.TutorialProjectPlayerState` _asbp_tutorial_project_player_state))

(event `self.BP_HealthComponent.OnOwnerDied`
  (bind _mesh (`self.Mesh`))
  (set `self.IsDied` true)
  (`self.DisableInput` (`GameplayStatics.GetPlayerController` 0) null)
  (set `SpringArmComponent.bDoCollisionTest` false (`self.SpringArm`))
  (`PrimitiveComponent.SetCollisionEnabled` (`self.CapsuleComponent`) "NoCollision")
  (`PrimitiveComponent.SetCollisionEnabled` _mesh "QueryAndPhysics")
  (`PrimitiveComponent.SetSimulatePhysics` _mesh true)
  (`self.SetLifeSpan` 3.0))

(event `self.CapsuleComponent.OnComponentBeginOverlap`
  (params (OverlappedComponent :type "PrimitiveComponent Object Reference") (OtherActor :type "Actor Object Reference") (OtherComp :type "PrimitiveComponent Object Reference") (OtherBodyIndex :type Integer) (bFromSweep :type Boolean) (SweepResult :type "HitResult Structure (by ref)"))
  (if (`KismetSystemLibrary.DoesImplementInterface` OtherActor "/Game/TutorialWork/Blueprints/Interfaces/BPI_Interactable.BPI_Interactable_C")
    (set `self.CurrentInteract` OtherActor)))

(event `EnhancedInput|/Game/TutorialWork/Core/EnhancedInput/Action/IA_TutorialProjectInteract`
  (params (ActionValue :type Boolean) (ElapsedSeconds :type "Float (double-precision)") (TriggeredSeconds :type "Float (double-precision)") (InputAction :type "InputAction Object Reference" :default "/Game/TutorialWork/Core/EnhancedInput/Action/IA_TutorialProjectInteract.IA_TutorialProjectInteract"))
  (:`Triggered`
    (bind _currentinteract (`self.CurrentInteract`)
      (:`then`
        (message `/Game/TutorialWork/Blueprints/Interfaces/BPI_Interactable.Interact` _currentinteract))
      (:`else`))))

(event `/Game/TutorialWork/Blueprints/Interfaces/BPI_Scorable.AddScore`
  (bind _tutorialprojectplayerstate (`self.TutorialProjectPlayerState`))
  (bind _result (`/Engine/EditorBlueprintResources/StandardMacros.IncrementInt` (`/Game/TutorialWork/Core/PlayerState/BP_TutorialProjectPlayerState.GetPlayerScore` _tutorialprojectplayerstate))
    (:`  `
      (`/Game/TutorialWork/Core/PlayerState/BP_TutorialProjectPlayerState.SetPlayerScore` _tutorialprojectplayerstate _result))))

(event `/Game/TutorialWork/Blueprints/Interfaces/BPI_Scorable.CollectCoin`
  (`self.CollectCoinDispatcher`))

(fn `UserConstructionScript`)